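; Player ship pawn for a bullet-hell game, handling movement, held-fire shooting, damage and death.
; The construction script loads stats, mesh, materials, hitboxes and fire point from a DT_Player row.
; Looping timers drive input-based mesh banking and BP_Bullet spawning, with a negative start delay offsetting the first shot's wait.
; Damage clamps health, plays random sounds and fires dispatchers; zero health disables input and hides the collider hierarchy.
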(event Custom|Event%20UpdateRotation
  ;[0 0 0] Event UpdateRotation
  (Transformation|SetRelativeRotation (Variables|Default|GetMeshContainer) (Math|Interpolation|RInterpTo (Variables|/Script/Engine.SceneComponent|GetRelativeRotation (Variables|Default|GetMeshContainer)) (Math|Rotator|MakeRotator (* (Math|Float|Clamp(Float) (.y (Variables|Private|Movement|GetNewMovement)) -1.0) 42.0) 0.0 0.0) (Variables|Private|GetUpdateDeltaTime) 6.0) false false))

(event EventBeginPlay
  ;[0 0 0] Event BeginPlay
  (Utilities|Time|SetTimerbyEvent (EventDispatchers|CreateEvent :!event Custom|Event%20UpdateRotation) (Variables|Private|GetUpdateDeltaTime) true))

(event Custom|Event%20Shoot
  (bind _firedirection (Variables|Default|GetFireDirection))
  (bind _returnvalue (Transformation|GetWorldTransform _firedirection))
  ;[0 0 0] Event Shoot
  (Game|SpawnActorfromClass "/Game/BulletHellEditor/Blueprints/Bullet/BP_Bullet.BP_Bullet_C" (Math|Transform|MakeTransform (.location _returnvalue) (.rotation _returnvalue) "1,1,1") "Undefined" 0 (Utilities|Struct|MakeDataTableRowHandle "/Game/BulletHellEditor/DataTables/DT_Bullet.DT_Bullet" "PlayerBullet") 0))

(event Input|ActionEvents|InputActionShoot
  (params (Key :type Key%20Structure))
  (bind _data (Variables|Private|GetData))
  (bind _shootingspeed (Utilities|Struct|BreakST_Player _data))
  ;[0 0 0] Event Shoot
  (:Pressed
    (bind _returnvalue (Utilities|Time|SetTimerbyEvent (delegate Custom|Event%20Shoot) _shootingspeed true (* _shootingspeed -1.0)))
    (Variables|Private|Shooting|SetShootTimer _returnvalue))
  (:Released
    (Utilities|Time|ClearandInvalidateTimerbyHandle (Variables|Private|Shooting|GetShootTimer))))

(event Input|AxisEvents|InputAxisHorizontalMovement
  (params (AxisValue :type Float%20%28single-precision%29))
  ;[0 0 0] Movement
  (bind _output_get (Variables|Private|Movement|SetNewMovement (Math|Vector2D|MakeVector2D (.x (Variables|Private|Movement|GetNewMovement)) AxisValue)))
  (Pawn|Input|AddMovementInput (Math|Vector|MakeVector (.x _output_get) 0.0 0.0) 1.0 false))

(event Input|AxisEvents|InputAxisVerticalMovement
  (params (AxisValue :type Float%20%28single-precision%29))
  ;[0 0 0] Movement
  (bind _output_get (Variables|Private|Movement|SetNewMovement (Math|Vector2D|MakeVector2D AxisValue (.y (Variables|Private|Movement|GetNewMovement)))))
  (Pawn|Input|AddMovementInput (Math|Vector|MakeVector 0.0 (.y _output_get) 0.0) 1.0 false))

(event EventTakeDamage
  (params (ImpactDamage :type Integer))
  ;[0 0 0] Event OnTakeDamage
  (Default|CallOnTakeDamage)
  (bind _structout (Utilities|Struct|SetmembersinST_Player (Variables|Private|GetData) (Math|Integer|Clamp(Integer) (- (.Health (Utilities|Struct|BreakST_Player (Variables|Private|GetData))) ImpactDamage) 0 (Variables|Private|GetMaxHealth))))
  (Default|CallOnHealthUpdate (/ (Math|Conversions|ToFloat(Integer) (.Health (Utilities|Struct|BreakST_Player _structout))) (Math|Conversions|ToFloat(Integer) (Variables|Private|GetMaxHealth))))
  (Audio|PlaySound2D (.OutItem (Utilities|Array|Random (.TakeDamageSounds (Utilities|Struct|BreakST_Player (Variables|Private|GetData))))) 1.0 1.0 0.0 0 0)
  (if (and (== (.Health (Utilities|Struct|BreakST_Player (Variables|Private|GetData))) 0) (not (Variables|Private|GetIsDead)))
    (Variables|Private|SetIsDead true)
    (CallFunction|Die)))

(event EventDie
  ;[0 0 0] Event Die
  (Default|CallOnDeath)
  (Audio|PlaySound2D (.OutItem (Utilities|Array|Random (.DeathSounds (Utilities|Struct|BreakST_Player (Variables|Private|GetData))))) 1.0 1.0 0.0 0 0)
  (Input|DisableInput (Game|GetPlayerController 0))
  (Rendering|SetVisibility (Variables|Default|GetCollider) false true))

(fn ConstructionScript
  (bind _data (Variables|Private|GetData))
  (bind _staticmesh (Utilities|Struct|BreakST_Player _data))
  (bind (_staticmesh_2 _materials _location _rotation _scale) (Utilities|Struct|BreakST_Model _staticmesh))
  ;[0 0 0] Load Data
  (bind _success (CallFunction|ReadDataTable))
  (if _success
    (|SetHitboxes)
    (Variables|Private|SetMaxHealth (.Health (Utilities|Struct|BreakST_Player (Variables|Private|GetData))))
    (Variables|/Script/Engine.FloatingPawnMovement|SetMaxSpeed (Variables|Default|GetFloatingPawnMovement) (.Speed (Utilities|Struct|BreakST_Player (Variables|Private|GetData))))
    (Components|StaticMesh|SetStaticMesh (Variables|Default|GetStaticMesh) _staticmesh_2)
    (Transformation|SetRelativeTransform (Variables|Default|GetStaticMesh) (Math|Transform|MakeTransform _location _rotation _scale) false false)
    (Transformation|SetRelativeLocation (Variables|Default|GetFireDirection) (.FireLocation (Utilities|Struct|BreakST_Player (Variables|Private|GetData))) false false)
    (|SetSkinMaterials)))

(fn ReadDataTable
  (bind _returnvalue (Utilities|GetDataTableRow "/Game/BulletHellEditor/DataTables/DT_Player.DT_Player" (.rowname (Variables|Public|GetID)))
    (:then
      (Variables|Private|SetData _returnvalue)
      (return true))
    (:RowNotFound
      (return false))))