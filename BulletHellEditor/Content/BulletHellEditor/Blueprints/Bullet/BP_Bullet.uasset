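; BP_Bullet is a data-driven projectile for a bullet hell game, configured from its DT_Bullet row.
; The construction script loads that row to set mesh, scale and materials; BeginPlay plays the spawn sound, sets the target collision channel to overlap and starts a looping timer and optional size-pulse timeline.
; Update moves it along its arrow and destroys it off-screen.
; Overlapping an actor implementing BI_DamagableActor sends damage and destroys the bullet.
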(event Custom|Event%20Update
  ;[0 0 0] Event Update
  (Transformation|AddActorWorldOffset (* (Math|Vector|GetForwardVector (Variables|Default|GetArrow)) (* (Variables|Private|GetDeltaTime) (.MovementSpeed (Utilities|Struct|BreakST_Bullet (Variables|Private|SettedinGame|GetData))))))
  (|CheckViewportLimits))

(event EventBeginPlay
  ;[0 0 0] Event BeginPlay
  (Audio|PlaySound2D (.SpawnSound (Utilities|Struct|BreakST_Bullet (Variables|Private|SettedinGame|GetData))) 1.0 1.0 0.0 0 0)
  (Utilities|Time|SetTimerbyEvent (EventDispatchers|CreateEvent :!event Custom|Event%20Update) (Variables|Private|GetDeltaTime) true)
  (Collision|SetCollisionResponsetoChannel (Variables|Default|GetStaticMesh) (.TargetCollisionType (Utilities|Struct|BreakST_Bullet (Variables|Private|SettedinGame|GetData))) "ECR_Overlap")
  (|IncreaseAnimation))

(event OnComponentBeginOverlap(StaticMesh)
  (params (OverlappedComponent :type Primitive%20Component%20Object%20Reference) (OtherActor :type Actor%20Object%20Reference) (OtherComp :type Primitive%20Component%20Object%20Reference) (OtherBodyIndex :type Integer) (bFromSweep :type Boolean) (SweepResult :type Hit%20Result%20Structure%20%28by%20ref%29))
  ;[0 0 0] Event OnBeginOverlap
  (if (Utilities|DoesObjectImplementInterface OtherActor "/Game/BulletHellEditor/Blueprints/Interfaces/BI_DamagableActor.BI_DamagableActor_C")
    (Class|BIDamagableActor|TakeDamage(Message) OtherActor (.Damage (Utilities|Struct|BreakST_Bullet (Variables|Private|SettedinGame|GetData))))
    (Actor|DestroyActor)))

(fn ConstructionScript
  ;[0 0 0] Load Data
  (bind _success (CallFunction|ReadDataTable))
  (if _success
    (Transformation|SetRelativeScale3D (Variables|Default|GetStaticMesh) (.Scale (Utilities|Struct|BreakST_Model (.StaticMesh (Utilities|Struct|BreakST_Bullet (Variables|Private|SettedinGame|GetData))))))
    (Components|StaticMesh|SetStaticMesh (Variables|Default|GetStaticMesh) (.StaticMesh (Utilities|Struct|BreakST_Model (.StaticMesh (Utilities|Struct|BreakST_Bullet (Variables|Private|SettedinGame|GetData))))))
    (|SetMaterials)))

(fn ReadDataTable
  (bind _returnvalue (Utilities|GetDataTableRow "/Game/BulletHellEditor/DataTables/DT_Bullet.DT_Bullet" (.rowname (Variables|Public|GetID)))
    (:then
      (Variables|Private|SettedinGame|SetData _returnvalue)
      (return true))
    (:RowNotFound
      (return false))))