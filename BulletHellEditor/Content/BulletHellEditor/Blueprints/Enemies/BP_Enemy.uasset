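; Data-driven enemy ship for a space shooter that hurts the player on contact and awards points when killed.
; Construction loads its DT_Enemy row to set mesh, materials and fire location.
; BeginPlay scales it in, runs the row's behavior tree and optional rotate sequence, while Tick can aim it at the player.
; Damage flashes dynamic materials, and death stops AI, shows score, plays effects and hides the mesh without destroying the actor.
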(event OnComponentBeginOverlap(StaticMesh)
  (params (OverlappedComponent :type Primitive%20Component%20Object%20Reference) (OtherActor :type Actor%20Object%20Reference) (OtherComp :type Primitive%20Component%20Object%20Reference) (OtherBodyIndex :type Integer) (bFromSweep :type Boolean) (SweepResult :type Hit%20Result%20Structure%20%28by%20ref%29))
  ;[0 0 0] Event OnComponentBeginOverlap
  (if (Variables|Private|GetSpawned)
    (bind _asbp_player_character (Utilities|Casting|CastToBP_PlayerCharacter OtherActor))
    (Default|TakeDamage _asbp_player_character 1)
    (CallFunction|Die)))

(event EventTick
  (params (DeltaSeconds :type Float%20%28single-precision%29))
  ;[0 0 0] Event Tick
  (switch Utilities|FlowControl|Switch|SwitchonE_EnemySight (.Sight (Utilities|Struct|BreakST_Enemy (Variables|Private|GetData)))
    (:NewEnumerator1
      (Transformation|SetWorldRotation (Variables|Default|GetMeshes) (Math|Rotator|FindLookatRotation (Transformation|GetWorldLocation (Variables|Default|GetMeshes)) (Transformation|GetActorLocation (Game|Player|GetPlayerPawn 0))) false false))))

(event EventBeginPlay
  ;[0 0 0] Event BeginPlay
  (Utilities|FlowControl|Sequence
    (:then_0
      (|GetShipMaterials))
    (:then_1
      (|Spawn))
    (:then_2
      (|GetPlayerReference))
    (:then_3
      (Components|Animation|SetAnimation))
    (:then_4
      (|RunAI))))

(event EventDamageMaterial
  ;[0 0 0] Event DamageMaterial
  (for _array_element (Variables|Private|GetMaterials)
    (Rendering|Material|SetVectorParameterValue _array_element "Color" "(R=1.000000,G=0.467914,B=0.141020,A=1.000000)" :!class /Script/Engine.MaterialInstanceDynamic)
    (Rendering|Material|SetScalarParameterValue _array_element "Emissive" 6.0 :!class /Script/Engine.MaterialInstanceDynamic))
  (Utilities|Time|SetTimerbyEvent (delegate EventEndDamageMaterial) 0.3))

(event EventEndDamageMaterial
  ;[0 0 0] Event DamageMaterial
  (for _array_element (Variables|Private|GetMaterials)
    (Rendering|Material|SetVectorParameterValue _array_element "Color" "(R=1.000000,G=0.462303,B=0.000000,A=1.000000)" :!class /Script/Engine.MaterialInstanceDynamic)
    (Rendering|Material|SetScalarParameterValue _array_element "Emissive" 7.0 :!class /Script/Engine.MaterialInstanceDynamic)))

(event EventTakeDamage
  (params (ImpactDamage :type Integer))
  ;[0 0 0] Event TakeDamage
  (Utilities|Struct|SetmembersinST_Enemy (Variables|Private|GetData) (- (.Health (Utilities|Struct|BreakST_Enemy (Variables|Private|GetData))) ImpactDamage))
  (Audio|PlaySound2D "/Game/BulletHellEditor/Sounds/Wav/Hit_Hurt6.Hit_Hurt6" 1.0 1.0 0.0 0 0)
  (if (<= (.Health (Utilities|Struct|BreakST_Enemy (Variables|Private|GetData))) 0)
    (CallFunction|Die)
    (else
      (CallFunction|DamageMaterial))))

(event EventDie
  ;[0 0 0] Event Die
  (Default|CallOnDeath)
  (|UpdateScore)
  (AI|Logic|StopLogic (Variables|/Script/AIModule.AIController|GetBrainComponent (AI|GetAIController self)) "")
  (|PlayVisualEffects)
  (|PlayAudio)
  (Collision|SetCollisionEnabled (Variables|Default|GetStaticMesh) "NoCollision")
  (Rendering|SetVisibility (Variables|Default|GetStaticMesh) false false)
  ;;[0.08763 0.09184 0.2135 1 14] FreezeMaterialEffect
  (bind _alpha (Timeline|T_DestroyedMaterial PlayFromStart)
    (:Update
      (for _array_element (Variables|Private|GetDestructibleMaterials)
        (Rendering|Material|SetVectorParameterValue _array_element "Color" (Math|Color|Lerp(LinearColor) :A "(R=1.000000,G=0.412325,B=0.000000,A=1.000000)" :Alpha _alpha) :!class /Script/Engine.MaterialInstanceDynamic)
        (Rendering|Material|SetScalarParameterValue _array_element "Emissive" (Math|Float|Lerp 4.0 0.0 _alpha) :!class /Script/Engine.MaterialInstanceDynamic)))))

(fn ConstructionScript
  ;[0 0 0] Load Data
  (bind _success (CallFunction|ReadDataTable))
  (if _success
    (ConstructionScript|ImplementData)))

(fn ImplementData
  ;[0 0 0] ImplementData
  (|SetTransform)
  (Utilities|FlowControl|Sequence
    (:then_0
      ;;[0.2708 0.08536 0.1663 1 14] StaticMesh
      (Components|StaticMesh|SetStaticMesh (Variables|Default|GetStaticMesh) (.StaticMesh (Utilities|Struct|BreakST_Model (.StaticMesh (Utilities|Struct|BreakST_Enemy (Variables|Private|GetData))))))
      (for (_ _array_index) (Rendering|Material|GetMaterials (Variables|Default|GetStaticMesh))
        (Rendering|Material|SetMaterial (Variables|Default|GetStaticMesh) _array_index (Utilities|Array|Get(acopy) (.Materials (Utilities|Struct|BreakST_Model (.StaticMesh (Utilities|Struct|BreakST_Enemy (Variables|Private|GetData))))) _array_index))))
    (:then_1
      ;;[0.3542 0.1662 0.07647] FireLocation
      (Transformation|SetRelativeLocation (Variables|Default|GetFireDirection) (.FireLocation (Utilities|Struct|BreakST_Enemy (Variables|Private|GetData))) false false))))

(fn ReadDataTable
  (bind _returnvalue (Utilities|GetDataTableRow "/Game/BulletHellEditor/DataTables/DT_Enemy.DT_Enemy" (.rowname (Variables|Public|GetID)))
    (:then
      (Variables|Private|SetData _returnvalue)
      (return true))
    (:RowNotFound
      (return false))))