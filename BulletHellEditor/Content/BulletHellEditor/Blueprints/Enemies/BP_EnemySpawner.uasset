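; Enemy spawner actor that places BP_Enemy instances at random points inside its Box volume.
; BeginPlay starts a looping timer with a negative start delay to shorten the wait before the first firing.
; The SpawnEnemy event picks a random DT_Enemy row and passes it to the new enemy as its ID, spawning it with a fixed rotation.
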(event Custom|Event%20SpawnEnemy
  (bind _box (Variables|Default|GetBox))
  ;[0 0 0] Event SpawnEnemy
  (bind _outrownames (DataTable|GetDataTableRowNames "/Game/BulletHellEditor/DataTables/DT_Enemy.DT_Enemy"))
  (Game|SpawnActorfromClass "/Game/BulletHellEditor/Blueprints/Enemies/BP_Enemy.BP_Enemy_C" (Math|Transform|MakeTransform (Math|Random|RandomPointinBoundingBox (Transformation|GetWorldLocation _box) (Components|Box|GetScaledBoxExtent _box)) "0,180.000000, 0" "1,1,1") "Undefined" 0 (Utilities|Struct|MakeDataTableRowHandle "/Game/BulletHellEditor/DataTables/DT_Enemy.DT_Enemy" (.OutItem (Utilities|Array|Random _outrownames))) 0))

(event EventBeginPlay
  ;[0 0 0] Event BeginPlay
  (bind _returnvalue (Utilities|Time|SetTimerbyEvent (EventDispatchers|CreateEvent :!event Custom|Event%20SpawnEnemy) 4.5 true -4.0))
  (Variables|Default|SetTimer _returnvalue))

(fn ConstructionScript)